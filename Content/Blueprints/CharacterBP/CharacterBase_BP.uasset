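; Base 2D flipbook character with point-and-click movement on the XZ plane, plus keyboard movement along X.
; Held mouse buttons open Tick gates for simple nav moves: left targets a pawn or point, right only points, with walk speed set by X distance.
; CancelPath halts movement and briefly suspends mouse input; Tab cycles global time dilation.
; Velocity drives idle/walk flipbook and sprite facing.
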(event `self.ReceiveBeginPlay`
  (set `PlayerController.bShowMouseCursor` true (`GameplayStatics.GetPlayerController` 0))
  (set `self.MouseInput?` true)
  (set `CharacterMovementComponent.MaxWalkSpeed` 100.0 (`self.CharacterMovement`))
  (`GameplayStatics.SetGlobalTimeDilation` 1.0))

(event `self.ReceiveTick`
  (params (DeltaSeconds :type "Float (single-precision)"))
  (bind _mouseinput_ (`self.MouseInput?`))
  (`|ExecutionSequence`
    (:`then_0`
      (`self.UpdateFlipbook`)
      (`self.UpdateRotation`))
    (:`then_1`
      ;[1 1 1] MouseInputMovement
      (if _mouseinput_
        (`/Engine/EditorBlueprintResources/StandardMacros.Gate` true :!label _label
          (:`Exit`
            (bind _actor (`self.GetClickedActor`))
            (`/Engine/EditorBlueprintResources/StandardMacros.IsValid` _actor
              (:`Is Valid`
                (`self.MoveToActor` _actor))
              (:`Is Not Valid`
                (`self.MoveToClickedPoint`)))))))
    (:`then_2`
      (if _mouseinput_
        (`/Engine/EditorBlueprintResources/StandardMacros.Gate` true :!label _label_2
          (:`Exit`
            (`self.MoveToClickedPoint`)))))))

(event `Key|LeftMouseButton`
  (params (Key :type "Key Structure"))
  ;[1 1 1] MouseInputMovement
  (:`Pressed`
    (goto _label :!via `Open`))
  (:`Released`
    (goto _label :!via `Close`)))

(event `Key|RightMouseButton`
  (params (Key :type "Key Structure"))
  ;[1 1 1] MouseInputMovement
  (:`Pressed`
    (goto _label_2 :!via `Open`))
  (:`Released`
    (goto _label_2 :!via `Close`)))

(event `InputAction|CancelPath`
  (params (Key :type "Key Structure"))
  ;[1 1 1] KeyboardInputMovement
  (:`Pressed`
    (`MovementComponent.StopMovementImmediately` (`self.CharacterMovement`))
    (set `self.MouseInput?` false))
  (:`Released`
    (`KismetSystemLibrary.Delay` 0.2)
    (set `self.MouseInput?` true)))

(event `InputAxis|MovementKeyboard`
  (params (AxisValue :type "Float (single-precision)"))
  ;[1 1 1] KeyboardInputMovement
  (`self.AddMovementInput` (1.0 0.0 0.0) AxisValue))

(event `Key|Tab`
  (params (Key :type "Key Structure"))
  ;[1 1 1] SetTimeDilation
  (:`Pressed`
    (`/Engine/EditorBlueprintResources/StandardMacros.CompareFloat` (`self.TimeSpeed`) 1.0
      (:`>`
        (set `self.TimeSpeed` 0.35))
      (:`==`
        (set `self.TimeSpeed` 2.2))
      (:`<`
        (set `self.TimeSpeed` 1.0)))
    (`GameplayStatics.SetGlobalTimeDilation` (`self.TimeSpeed`))))

(fn `GetClickedActor`
  (returns (Actor :type "Actor Object Reference"))
  (return (`.HitActor` (`GameplayStatics.BreakHitResult` (`PlayerController.GetHitResultUnderCursorForObjects` (`GameplayStatics.GetPlayerController` 0) (`|MakeArray` "ObjectTypeQuery3" :!type "EObjectTypeQuery Enum") true)))))

(fn `GetDestionationToMove`
  (returns (Destionation :type "Vector Structure"))
  (bind _hitresult (`PlayerController.GetHitResultUnderCursorByChannel` (`GameplayStatics.GetPlayerController` 0) "TraceTypeQuery1" true))
  (return (`KismetMathLibrary.MakeVector` (.x (`.Location` (`GameplayStatics.BreakHitResult` _hitresult))) 0.0 (.z (`.Location` (`GameplayStatics.BreakHitResult` _hitresult))))))

(fn `MoveToActor`
  (params (Actor :type "Actor Object Reference"))
  (`AIBlueprintHelperLibrary.SimpleMoveToActor` (`GameplayStatics.GetPlayerController` 0) Actor))

(fn `MoveToClickedPoint`
  (locals (MoveDestionation :type "Vector Structure"))
  (bind _returnvalue_x (`KismetMathLibrary.BreakVector` (`self.K2_GetActorLocation`)))
  (bind _movedestionation_x (`KismetMathLibrary.BreakVector` (`local.MoveDestionation`)))
  (bind _charactermovement (`self.CharacterMovement`))
  (bind _destionation (`self.GetDestionationToMove`))
  (set `local.MoveDestionation` _destionation)
  (if (not (== (`local.MoveDestionation`) (0.0 0.0 0.0)))
    (if (> (`KismetMathLibrary.Abs` (- _movedestionation_x _returnvalue_x)) 50.0)
      (set `CharacterMovementComponent.MaxWalkSpeed` 100.0 _charactermovement)
      (else
        (set `CharacterMovementComponent.MaxWalkSpeed` 50.0 _charactermovement)))
    (`AIBlueprintHelperLibrary.SimpleMoveToLocation` (`GameplayStatics.GetPlayerController` 0) (`local.MoveDestionation`))))

(fn `UpdateFlipbook`
  (locals (AnimationState :type "/Game/Blueprints/CharacterBP/FlipbooksState_E Enum"))
  (set `local.AnimationState` (select `bool` (!= (`KismetMathLibrary.VSize` (`self.GetVelocity`)) 0.0) :`false` "NewEnumerator2" :`true` "NewEnumerator1" :!type "/Game/Blueprints/CharacterBP/FlipbooksState_E Enum"))
  (`PaperFlipbookComponent.SetFlipbook` (`self.Sprite`) (select `/Game/Blueprints/CharacterBP/FlipbooksState_E` (`local.AnimationState`) :`NewEnumerator1` "/Game/Assets/Flipbooks/Walk_FB.Walk_FB" :`NewEnumerator2` "/Game/Assets/Flipbooks/Idle_FB.Idle_FB" :`NewEnumerator3` "/Game/Assets/Flipbooks/Walk_FB.Walk_FB" :!type "PaperFlipbook Object Reference")))

(fn `UpdateRotation`
  (bind _returnvalue_x (`KismetMathLibrary.BreakVector` (`self.GetVelocity`)))
  (bind _sprite (`self.Sprite`))
  (`/Engine/EditorBlueprintResources/StandardMacros.CompareFloat` _returnvalue_x
    (:`>`
      (`SceneComponent.K2_SetRelativeRotation` :`self` _sprite))
    (:`<`
      (`SceneComponent.K2_SetRelativeRotation` _sprite (struct :`Yaw` 180.0) false false))))

(fn `UserConstructionScript`)