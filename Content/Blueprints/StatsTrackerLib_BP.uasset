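; Blueprint function library that records and reads named game statistics stored in a Stats map on GameInstance_BP.
; GetStats fetches and casts the game instance, and the other functions use it to reach the map.
; AddStats accumulates a value onto an existing entry or creates it if absent, while ReadStats returns the stored value for a name.
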(fn `AddStats`
  (params (StatName :type String) (Value :type "Float (double-precision)"))
  (bind _gameinstance (`self.GetStats` null))
  (bind _stats (`/Game/Blueprints/GameInstance_BP.Stats` _gameinstance))
  (bind (_value _returnvalue) (`BlueprintMapLibrary.Map_Find` _stats (`local.StatName`)))
  (if _returnvalue
    (`BlueprintMapLibrary.Map_Add` _stats (`local.StatName`) (+ (`local.Value`) _value))
    (else
      (`BlueprintMapLibrary.Map_Add` _stats (`local.StatName`) (`local.Value`)))))

(fn `GetStats`
  (returns (GameInstance :type "/Game/Blueprints/GameInstance_BP Object Reference"))
  (bind _asgame_instance_bp (cast `/Game/Blueprints/GameInstance_BP` (`GameplayStatics.GetGameInstance` null)))
  (return _asgame_instance_bp))

(fn `ReadStats`
  (params (StatName :type String))
  (returns (Value :type "Float (double-precision)"))
  (bind _gameinstance (`self.GetStats` null))
  (return (`BlueprintMapLibrary.Map_Find` (`/Game/Blueprints/GameInstance_BP.Stats` _gameinstance) (`local.StatName`))))