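; WorldController is a controller for a Paper2D game where movement input rotates its controlled pawn, presumably the world, instead of moving the character.
; On BeginPlay it spawns a separate CharacterController and character, then has that controller possess the character.
; The Movement axis pitches the controlled pawn opposite to the input at WorldRotateSpeed.
; Tick reads the same input to switch walk or idle flipbooks and flip the character's facing.
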(event `self.ReceiveBeginPlay`
  (bind _returnvalue (`KismetMathLibrary.MakeTransform` (0.0 0.0 0.0)))
  (bind _returnvalue_2 (`|SpawnActorFromClass` "/Game/Blueprints/CharacterController.CharacterController_C" _returnvalue "Undefined" "OverrideRootScale" null null))
  (set `self.CharacterController` _returnvalue_2)
  (bind _returnvalue_3 (`|SpawnActorFromClass` "/Game/Blueprints/Character.Character_C" _returnvalue "Undefined" "OverrideRootScale" null null))
  (set `self.CharacterBase` _returnvalue_3)
  (`self.Possess` (`self.CharacterController`) (`self.CharacterBase`)))

(event `self.ReceiveTick`
  (params (DeltaSeconds :type "Float (single-precision)"))
  (`self.CharacterUpdateFlipbook`)
  (`self.CharacterUpdateRotation`))

(event `InputAxis|Movement`
  (params (AxisValue :type "Float (single-precision)"))
  (`self.WorldUpdateRotation`))

(fn `CharacterUpdateFlipbook`
  (bind _playerflipbook (`/Game/Blueprints/Character.PlayerFlipbook` (`self.CharacterBase`)))
  (if (!= (`self.GetInputAxisValue`) 0.0)
    (`PaperFlipbookComponent.SetFlipbook` _playerflipbook "/Game/Assets/Flipbooks/Player_Walk_FB.Player_Walk_FB")
    (else
      (`PaperFlipbookComponent.SetFlipbook` _playerflipbook "/Game/Assets/Flipbooks/Player_Idle_FB.Player_Idle_FB"))))

(fn `CharacterUpdateRotation`
  (bind _characterbase (`self.CharacterBase`))
  (`/Engine/EditorBlueprintResources/StandardMacros.CompareFloat` (`self.GetInputAxisValue`)
    (:`>`
      (`self.K2_SetActorRotation` _characterbase (struct :`Yaw` 180.0) false))
    (:`<`
      (`self.K2_SetActorRotation` :`self` _characterbase))))

(fn `UserConstructionScript`)

(fn `WorldUpdateRotation`
  (`self.K2_AddActorWorldRotation` (`self.K2_GetPawn`) (`KismetMathLibrary.MakeRotator` 0.0 (* (`self.WorldRotateSpeed`) (`self.GetInputAxisValue`) -1.0)) false false))